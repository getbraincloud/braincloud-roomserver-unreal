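; Player controller that hands a joining player's data and room passcode from the client to the server for validation.
; The client reads both from the GameManager game instance, cached through GetGameManager, and sends them to the server.
; The server writes them into BCPlayerState, then passes that state to BCGameMode to validate the player code.
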(event `Client_SendPlayerData`
  (bind _gamemanager (`self.GetGameManager`))
  (bind (_roomdata_lobbyid _roomdata_address _roomdata_portudp _roomdata_porttcp _roomdata_passcode) (break `/Game/Blueprints/Core/Data/RoomData` (`/Game/Blueprints/Core/GameManager.RoomData` _gamemanager)))
  (`self.Server_ReceivePlayerData` (`/Game/Blueprints/Core/GameManager.PlayerData` _gamemanager) _roomdata_passcode))

(event `Server_ReceivePlayerData`
  (params (PlayerData :type "/Game/Blueprints/Core/Data/PlayerData Structure") (Passcode :type String))
  (bind _asbcplayer_state (cast `/Game/Blueprints/Core/BCPlayerState` (`self.PlayerState`)))
  (set `/Game/Blueprints/Core/BCPlayerState.PlayerData` PlayerData _asbcplayer_state)
  (set `/Game/Blueprints/Core/BCPlayerState.passcode` Passcode _asbcplayer_state)
  (`self.Server_ValidatePlayerData`))

(event `Server_ValidatePlayerData`
  (bind _asbcplayer_state (cast `/Game/Blueprints/Core/BCPlayerState` (`self.PlayerState`)))
  (bind _asbcgame_mode (cast `/Game/Blueprints/Core/BCGameMode` (`GameplayStatics.GetGameMode`)))
  (`/Game/Blueprints/Core/BCGameMode.Server_ValidatePlayerCode` _asbcgame_mode _asbcplayer_state))

(fn `UserConstructionScript`)