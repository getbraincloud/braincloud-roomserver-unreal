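; Game mode for a brainCloud lobby-hosted dedicated-server shooter, running the match lifecycle, players and scoring.
; Server-to-server requests fetch lobby data, signal room ready, send keep-alives and report room stopped.
; Joining players are tracked and passcode-checked against lobby members, then spawned with pistols at random starts or kicked.
; A countdown ends the match, freezes players and returns them to the lobby; an emptied server starts a shutdown timer.
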(event `DestroyWeapon`
  (params (Player :type "/Game/Blueprints/BP_ThirdPersonCharacter Object Reference"))
  ;[1 0.5174 0.7801] Server functions
  ;;[1 1 1 0] Destroy player weapon
  (`self.K2_DestroyActor` (`/Game/Blueprints/BP_ThirdPersonCharacter.EquippedWeapon` Player)))

(event `Server_UpdateAllScoreboards`
  ;[1 0.5174 0.7801] Server functions
  ;;[1 1 1 0] Update scoreboards
  (for _array_element (`self.Players`)
    (bind _asbp_third_person_character (cast `/Game/Blueprints/BP_ThirdPersonCharacter` (`PlayerState.GetPawn` _array_element)))
    (`/Game/Blueprints/BP_ThirdPersonCharacter.Client_UpdateScoreboard` _asbp_third_person_character)))

(event `Multi_DisablePlayerMovements`
  ;[1 0.5174 0.7801] Server functions
  ;;[1 1 1 0] Disable player movements for end game screen
  (for _array_element (`self.Players`)
    (bind _asbp_third_person_character (cast `/Game/Blueprints/BP_ThirdPersonCharacter` (`PlayerState.GetPawn` _array_element)))
    (`CharacterMovementComponent.DisableMovement` (`Character.CharacterMovement` _asbp_third_person_character))
    (`WidgetBlueprintLibrary.SetInputMode_UIOnlyEx` (`PlayerState.GetPlayerController` _array_element) null)))

(event `self.ReceiveBeginPlay`
  ;[1 0.7956 0.4078] Startup server and get lobby data
  (`KismetArrayLibrary.Array_Clear` (`self.Players`))
  (add `self.OnLobbyDataUpdated` (delegate `OnLobbyDataUpdate`))
  (`self.GetLobbyData`))

(event `self.ReceiveTick`
  (params (DeltaSeconds :type "Float (single-precision)"))
  ;[1 1 1] Run brainCloud S2S callbacks
  (`self.RunCallbacks`))

(event `self.K2_PostLogin`
  (params (NewPlayer :type "PlayerController Object Reference"))
  ;[0.6903 1 0.7536] Handle player connected
  (`|ExecutionSequence`
    (:`then_0`
      (`KismetSystemLibrary.K2_ClearAndInvalidateTimerHandle` (`self.ServerTimeoutHandle`)))
    (:`then_1`
      (bind _asbc_player_controller (cast `/Game/Blueprints/Core/BC_PlayerController` NewPlayer))
      (`/Game/Blueprints/Core/BC_PlayerController.Client_SendPlayerData` _asbc_player_controller))
    (:`then_2`
      (`self.HandlePlayerConnected` (`Controller.PlayerState` NewPlayer))
      (`self.Server_UpdateAllScoreboards`))
    (:`then_3`
      (if (not (`KismetSystemLibrary.IsPackagedForDistribution`))
        (`self.RespawnPlayer` NewPlayer)))
    (:`then_4`
      (`self.SetAllOverheadNameText`))))

(event `RespawnPlayer`
  (params (PlayerController :type "Controller Object Reference"))
  ;[1 0.5174 0.7801] Server functions
  ;;[1 1 1 0] Handle player respawn
  (bind _asbp_third_person_character (cast `/Game/Blueprints/BP_ThirdPersonCharacter` (`Controller.K2_GetPawn` PlayerController))
    (:`then`
      (bind _isalive (`/Game/Blueprints/BP_ThirdPersonCharacter.GetIsAlive` _asbp_third_person_character))
      (if (not _isalive)
        (`self.DestroyWeapon` _asbp_third_person_character)
        (`self.K2_DestroyActor` _asbp_third_person_character)
        (`Controller.UnPossess` PlayerController)
        (bind _returnvalue (`|SpawnActorFromClass` "/Game/Blueprints/BP_ThirdPersonCharacter.BP_ThirdPersonCharacter_C" (`self.GetTransform` (`self.K2_FindPlayerStart` PlayerController)) "Undefined" "OverrideRootScale" null null :!label _label))
        (`/Game/Blueprints/BP_ThirdPersonCharacter.EquipPistol` _returnvalue)
        (`Controller.Possess` PlayerController _returnvalue)
        (`/Game/Blueprints/BP_ThirdPersonCharacter.Server_SetNameTag` _returnvalue)
        (`self.SetAllOverheadNameText`)))
    (:`CastFailed`
      (goto _label))))

(event `OnLobbyDataUpdate`
  ;[1 0.7956 0.4078] Startup server and get lobby data
  (`self.SetRoomIsReady`)
  (bind _returnvalue (`KismetSystemLibrary.K2_SetTimerDelegate` (`|CreateDelegate` :!event `OnGameTimeTick`) 1.0 true))
  (set `self.GameTimerHandle` _returnvalue)
  (bind _returnvalue_2 (`KismetSystemLibrary.K2_SetTimerDelegate` (`|CreateDelegate` :!event `SendKeepAlive`) (`self.KeepAliveRate`) true))
  (set `self.KeepAliveTimerHandle` _returnvalue_2)
  (remove `self.OnLobbyDataUpdated` (delegate `OnLobbyDataUpdate`)))

(event `Server_ValidatePlayerCode`
  (params (PlayerState :type "/Game/Blueprints/Core/BCPlayerState Object Reference"))
  ;[0.6562 1 1] Validate player passcode
  (add `self.OnLobbyDataUpdated` (delegate `Server_OnLobbyDataUpdated`))
  (`self.GetLobbyData`))

(event `Server_OnLobbyDataUpdated`
  ;[0.6562 1 1] Validate player passcode
  (`|ExecutionSequence`
    (:`then_0`
      (`/Engine/EditorBlueprintResources/StandardMacros.IsValid` (stale `Server_ValidatePlayerCode` PlayerState)
        (:`Is Valid`
          (bind _valid (`self.ValidatePlayer` (stale `Server_ValidatePlayerCode` PlayerState)))
          (if _valid
            (`self.RespawnPlayer` (`PlayerState.GetPlayerController` (stale `Server_ValidatePlayerCode` PlayerState)))
            (`KismetSystemLibrary.DelayUntilNextTick`)
            (`self.SetAllOverheadNameText`)
            (else
              (bind _asbp_third_person_character (cast `/Game/Blueprints/BP_ThirdPersonCharacter` (`PlayerState.GetPawn` (stale `Server_ValidatePlayerCode` PlayerState))))
              (`/Game/Blueprints/BP_ThirdPersonCharacter.GetKicked` _asbp_third_person_character "Invalid passcode"))))))
    (:`then_1`
      (remove `self.OnLobbyDataUpdated` (delegate `Server_OnLobbyDataUpdated`)))))

(event `OnPlayerDied`
  (params (Victim :type "/Game/Blueprints/Core/BCPlayerState Object Reference") (Attacker :type "/Game/Blueprints/Core/BCPlayerState Object Reference"))
  ;[1 0.5174 0.7801] Server functions
  ;;[1 1 1 0] Update stats on player death
  (set `/Game/Blueprints/Core/BCPlayerState.deaths` (+ (`/Game/Blueprints/Core/BCPlayerState.deaths` Victim) 1) Victim)
  (set `/Game/Blueprints/Core/BCPlayerState.scoreValue` (- (`/Game/Blueprints/Core/BCPlayerState.scoreValue` Victim) 50) Victim)
  (set `/Game/Blueprints/Core/BCPlayerState.kills` (+ (`/Game/Blueprints/Core/BCPlayerState.kills` Attacker) 1) Attacker)
  (set `/Game/Blueprints/Core/BCPlayerState.scoreValue` (+ (`/Game/Blueprints/Core/BCPlayerState.scoreValue` Attacker) 100) Attacker))

(event `self.K2_OnLogout`
  (params (ExitingController :type "Controller Object Reference"))
  ;[0.779 0.8343 1] Handle player disconnected
  (bind _asbp_third_person_character (cast `/Game/Blueprints/BP_ThirdPersonCharacter` (`Controller.K2_GetPawn` ExitingController))
    (:`then`
      (`self.DestroyWeapon` _asbp_third_person_character))
    (:`CastFailed`
      _))
  (`|ExecutionSequence`
    (:`then_0`
      (`self.GetLobbyData`)
      (`self.HandlePlayerDisconnected` (`Controller.PlayerState` ExitingController)))
    (:`then_1`
      (`KismetSystemLibrary.Delay` 0.5)
      (`self.Server_UpdateAllScoreboards`))
    (:`then_2`
      (`KismetSystemLibrary.Delay` 0.5)
      (`self.CheckServerEmpty`))))

(event `LobbyDataCallback`
  ;[1 1 1] Check if game lobby is empty - shutdown server if so
  (if (`KismetArrayLibrary.Array_IsEmpty` (`.Members_23_F310257D4A29316BF1E3278B40E1ECB0` (break `/Game/Blueprints/Core/Data/LobbyData` (`self.LobbyData`))))
    (`KismetSystemLibrary.PrintString` "No more players, shutting down...")
    (`KismetSystemLibrary.QuitGame` null "Quit" true)
    (else
      (remove `self.OnLobbyDataUpdated` (delegate `LobbyDataCallback`)))))

(event `TakePlayersToLobby`
  (bind _players (`self.Players`))
  ;[1 0.5174 0.7801] Server functions
  (`KismetSystemLibrary.PrintString` "[Take players to lobby]")
  (if (`KismetArrayLibrary.Array_IsNotEmpty` _players)
    (for _array_element _players
      (`/Engine/EditorBlueprintResources/StandardMacros.IsValid` _array_element
        (:`Is Valid`
          (`/Game/Blueprints/Core/BCPlayerState.Client_BackToLobby` _array_element))))
    (`KismetArrayLibrary.Array_Clear` _players)))

(fn `CheckForEmptyLobby`
  (add `self.OnLobbyDataUpdated` (`|CreateDelegate` :!event `LobbyDataCallback`))
  (`self.GetLobbyData`))

(fn `CheckServerEmpty`
  (locals (AllPlayersInvalid :type Boolean :default true))
  (bind _servertimeouthandle (`self.ServerTimeoutHandle`))
  (`KismetSystemLibrary.PrintString` "[Checking if server is empty]")
  (if (`KismetArrayLibrary.Array_IsEmpty` (`self.Players`))
    (`KismetSystemLibrary.PrintString` "Server is empty!")
    (if (`KismetSystemLibrary.K2_IsValidTimerHandle` _servertimeouthandle)
      (`KismetSystemLibrary.K2_ClearAndInvalidateTimerHandle` _servertimeouthandle))
    (bind _returnvalue (`KismetSystemLibrary.K2_SetTimerDelegate` (`|CreateDelegate` :!event `ShutdownServer`) 30.0))
    (set `self.ServerTimeoutHandle` _returnvalue)
    (`KismetSystemLibrary.PrintString` "Started shutdown timer 30 seconds")
    (else
      (`KismetSystemLibrary.PrintString` "Server is NOT empty"))))

(fn `EndGame`
  (`KismetSystemLibrary.PrintString` "[END GAME]")
  (`self.Multi_DisablePlayerMovements`)
  (bind _returnvalue (`KismetSystemLibrary.K2_SetTimer` null "OnRestartTimerTick" 1.0 true))
  (set `self.RestartTimerHandle` _returnvalue)
  (for _array_element (`self.Players`)
    (set `/Game/Blueprints/Core/BCPlayerState.GameOver` true _array_element)))

(fn `FindPlayerStart`
  (params (Player :type "Controller Object Reference") (IncomingName :type String))
  (returns (ReturnValue :type "Actor Object Reference"))
  (bind _outactors (`GameplayStatics.GetAllActorsOfClass` "/Script/Engine.PlayerStart"))
  (return (`|GetArrayItem` _outactors (`KismetMathLibrary.RandomIntegerInRange` 0 (- (`KismetArrayLibrary.Array_Length` _outactors) 1)))))

(fn `GetLobbyData`
  (if (`KismetSystemLibrary.IsDedicatedServer`)
    (`self.S2SRequest` (`KismetStringLibrary.Concat_StrStr` "{\"service\":\"lobby\", \"operation\":\"GET_LOBBY_DATA\", \"data\":{\"lobbyId\": \"" (`self.lobbyId`) "\"}}") (`|CreateDelegate` :!event `OnLobbyDataReceived`))
    (return)))

(fn `HandlePlayerConnected`
  (params (PlayerState :type "PlayerState Object Reference"))
  (bind _players (`self.Players`))
  (bind _asbcplayer_state (cast `/Game/Blueprints/Core/BCPlayerState` PlayerState)
    (:`then`
      (if (not (`KismetArrayLibrary.Array_Contains` _players _asbcplayer_state))
        (bind _returnvalue (`KismetArrayLibrary.Array_Add` _players _asbcplayer_state))
        (set `/Game/Blueprints/Core/BCPlayerState.netId` _returnvalue _asbcplayer_state))
      (`self.OnPlayerConnected` _asbcplayer_state)
      (`/Game/Blueprints/Core/BCPlayerState.UpdateConnectionStatus` _asbcplayer_state true)
      (return))
    (:`CastFailed`
      (return))))

(fn `HandlePlayerDisconnected`
  (params (PlayerState :type "PlayerState Object Reference"))
  (bind _players (`self.Players`))
  (`KismetSystemLibrary.PrintString` "[HandlePlayerDisconnected]")
  (bind _asbcplayer_state (cast `/Game/Blueprints/Core/BCPlayerState` PlayerState)
    (:`then`
      _)
    (:`CastFailed`
      (`KismetSystemLibrary.PrintString` "[HandlePlayerDisconnected failed to cast to BCPlayerState class instance]")))
  (if (`KismetArrayLibrary.Array_Contains` _players _asbcplayer_state)
    (`/Game/Blueprints/Core/BCPlayerState.UpdateConnectionStatus` _asbcplayer_state false)
    (bind _returnvalue (`KismetArrayLibrary.Array_RemoveItem` _players _asbcplayer_state))
    (if _returnvalue
      (`KismetSystemLibrary.PrintString` "[Removed player from players array]")
      (else
        (`KismetSystemLibrary.PrintString` "[Couldn't remove player from players array]")))
    (`self.K2_DestroyActor` _asbcplayer_state)
    (else
      (`KismetSystemLibrary.PrintString` "[HandlePlayerDisconnected player wasn't contained in players array]"))))

(fn `OnGameTimeTick`
  (bind _result (`/Engine/EditorBlueprintResources/StandardMacros.DecrementFloat` (`self.TotalGameSeconds`))
    (:`  `
      (bind _output_get (set `self.TotalGameSeconds` _result))
      (if (<= _output_get 0.0)
        (`self.EndGame`)
        (`KismetSystemLibrary.K2_ClearAndInvalidateTimerHandle` (`self.GameTimerHandle`))))))

(fn `OnKeepAliveResponse`
  (params (OutputString :type String))
  (`KismetSystemLibrary.PrintString` (`KismetStringLibrary.Concat_StrStr` "[KEEP ALIVE RESPONSE] " OutputString)))

(fn `OnLobbyDataReceived`
  (params (jsonData :type String))
  (locals (m_lobbyMembers :type "Array of /Game/Blueprints/Core/Data/LobbyMemberData Structure"))
  (bind _m_lobbymembers (`local.m_lobbyMembers`))
  (`KismetSystemLibrary.LogString` (`KismetStringLibrary.Concat_StrStr` "Received lobby data  \n" jsonData))
  (bind _outjsonobject (`JsonBlueprintFunctionLibrary.FromString` jsonData))
  (bind _outvalue (`|GetJsonField` _outjsonobject "status"))
  (if (== _outvalue 200)
    (`KismetArrayLibrary.Array_Clear` (`local.m_lobbyMembers`))
    (bind _outvalue_2 (`|GetJsonField` _outjsonobject "data"))
    (bind _outvalue_3 (`|GetJsonField` _outvalue_2 "lobbyType"))
    (bind _outvalue_4 (`|GetJsonField` _outvalue_2 "state"))
    (bind _outvalue_5 (`|GetJsonField` _outvalue_2 "rating"))
    (bind _outvalue_6 (`|GetJsonField` _outvalue_2 "ownerCxId"))
    (bind _outvalue_7 (`|GetJsonField` _outvalue_2 "keepAliveRateSeconds"))
    (set `self.KeepAliveRate` _outvalue_7)
    (bind _outvalue_8 (`|GetJsonField` _outvalue_2 "members"))
    (bind _asgame_manager (cast `/Game/Blueprints/Core/GameManager` (`GameplayStatics.GetGameInstance`)))
    (for _array_element _outvalue_8
      (bind _member_data (`/Game/Blueprints/Core/GameManager.ProcessLobbyMemberData` _asgame_manager _array_element))
      (`KismetArrayLibrary.Array_Add` _m_lobbymembers _member_data))
    (set `self.LobbyData` (make `/Game/Blueprints/Core/Data/LobbyData` (`self.lobbyId`) _outvalue_4 _outvalue_5 _outvalue_3 0 0 _outvalue_6 _m_lobbymembers))
    (`self.OnLobbyDataUpdated`)
    (else
      (`self.ShutdownServer`))))

(fn `OnPlayerDataReady`
  (params (PlayerState :type "/Game/Blueprints/Core/BCPlayerState Object Reference")))

(fn `OnRep_TotalGameSeconds`
  (for _array_element (`self.Players`)
    (`/Engine/EditorBlueprintResources/StandardMacros.IsValid` _array_element
      (:`Is Valid`
        (set `/Game/Blueprints/Core/BCPlayerState.GameTime` (`self.TotalGameSeconds`) _array_element)))))

(fn `OnRestartTimerTick`
  (bind _result (`/Engine/EditorBlueprintResources/StandardMacros.DecrementInt` (`self.RestartTimerSeconds`))
    (:`  `
      (if (<= _result 0)
        (`self.TakePlayersToLobby`)
        (`KismetSystemLibrary.K2_ClearAndInvalidateTimerHandle` (`self.RestartTimerHandle`))
        (`KismetSystemLibrary.PrintString` "[Timer cleared]")
        (`KismetSystemLibrary.K2_SetTimer` null "SendRoomStopped" 1.0)
        (`KismetSystemLibrary.PrintString` "[SendRoomStopped timer set - 1 second]")))))

(fn `OnRoomReadyCallback`
  (params (OutputString :type String)))

(fn `OnRoomStoppedCallback`
  (params (OutputString :type String))
  (`KismetSystemLibrary.PrintString` (`KismetStringLibrary.Concat_StrStr` "[ROOMSTOPPED RESPONSE] " OutputString))
  (`self.ShutdownServer`))

(fn `RestartGame`
  (`/Engine/EditorBlueprintResources/ActorMacros.Switch Has Authority`
    (:`Authority`
      (`KismetSystemLibrary.ExecuteConsoleCommand` (`KismetStringLibrary.Concat_StrStr` "ServerTravel " "Stylized_Egypt_Demo") null))))

(fn `SendKeepAlive`
  (if (`KismetSystemLibrary.IsDedicatedServer`)
    (`self.S2SRequest` (`KismetStringLibrary.Concat_StrStr` "{\"service\":\"lobby\", \"operation\":\"SYS_ROOM_KEEP_ALIVE\", \"data\":{\"lobbyId\":\"" (`self.lobbyId`) "\"}}") (`|CreateDelegate` :!event `OnKeepAliveResponse`))))

(fn `SendRoomStopped`
  (bind _returnvalue (`KismetStringLibrary.Concat_StrStr` "{\"service\":\"lobby\", \"operation\":\"SYS_ROOM_STOPPED\", \"data\":{\"lobbyId\":\"" (`self.lobbyId`) "\"}}"))
  (`KismetSystemLibrary.PrintString` (`KismetStringLibrary.Concat_StrStr` "[SEND ROOM STOPPED] " _returnvalue))
  (`self.S2SRequest` _returnvalue (`|CreateDelegate` :!event `OnRoomStoppedCallback`)))

(fn `SetAllOverheadNameText`
  (for _array_element (`self.Players`)
    (`/Game/Blueprints/Core/BCPlayerState.Server_SetOverheadTextData` _array_element)))

(fn `SetRoomIsReady`
  (if (`KismetSystemLibrary.IsDedicatedServer`)
    (`self.S2SRequest` (`KismetStringLibrary.Concat_StrStr` "{\"service\":\"lobby\", \"operation\":\"SYS_ROOM_READY\", \"data\":{\"lobbyId\":\"" (`self.lobbyId`) "\"}}") (`|CreateDelegate` :!event `OnRoomReadyCallback`))))

(fn `UpdatePlayerScoreboard`
  (params (BCPlayerState :type "/Game/Blueprints/Core/BCPlayerState Object Reference"))
  (bind _returnvalue (`PlayerState.GetPawn` BCPlayerState))
  (`/Engine/EditorBlueprintResources/StandardMacros.IsValid` _returnvalue
    (:`Is Valid`
      (bind _asbp_third_person_character (cast `/Game/Blueprints/BP_ThirdPersonCharacter` _returnvalue))
      (`/Game/Blueprints/BP_ThirdPersonCharacter.UpdateScoreboard` _asbp_third_person_character))))

(fn `UserConstructionScript`)

(fn `ValidatePlayer`
  (params (playerState :type "/Game/Blueprints/Core/BCPlayerState Object Reference"))
  (returns (valid :type Boolean))
  (bind _passcode (`/Game/Blueprints/Core/BCPlayerState.passcode` playerState))
  (for _array_element (`.Members_23_F310257D4A29316BF1E3278B40E1ECB0` (break `/Game/Blueprints/Core/Data/LobbyData` (`self.LobbyData`)))
    (bind ((`CxId_17_921E40064DDD89563539C68EFFCA3E6F` _cxid) (`Passcode_20_492B6F134DF6C0C0C3EA7982B119244F` _passcode_2)) (break `/Game/Blueprints/Core/Data/LobbyMemberData` _array_element))
    ;[1 1 1] Player Found?
    (if (`KismetStringLibrary.EqualEqual_StrStr` _cxid (`.CxId_17_921E40064DDD89563539C68EFFCA3E6F` (break `/Game/Blueprints/Core/Data/LobbyMemberData` (`.LobbyMemberData_22_540CFA8F433D9AFCAF915C8E0BF041E1` (break `/Game/Blueprints/Core/Data/PlayerData` (`/Game/Blueprints/Core/BCPlayerState.PlayerData` playerState))))))
      (`KismetSystemLibrary.LogString` (`KismetStringLibrary.Concat_StrStr` "player code: " _passcode "server code: " _passcode_2))
      ;[1 1 1] Has valid passcode?
      (if (`KismetStringLibrary.EqualEqual_StrStr` _passcode_2 _passcode)
        (return true)
        (else
          (return false)))))
  (return false))