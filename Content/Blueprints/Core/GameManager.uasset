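; Game manager that runs the brainCloud session: SDK initialization, RTT friend presence, logout and lobby matchmaking.
; Create, join and find requests use ping data and register RTT lobby callbacks that feed HandleLobbyCallbacks.
; That handler parses JSON into lobby, member and room structs and drives MainUIWidget screens and states.
; ROOM READY triggers a console "open" to the assigned server's address and UDP port.
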(event `self.ReceiveInit`
  ;[0.3698 0.3794 0.6771 0.688] Initialize and Run brainCloud
  (`self.InitializeBrainCloud`)
  (`KismetSystemLibrary.K2_SetTimerDelegate` (delegate `OnBCInitialized`) 0.0001 true 0.01))

(event `self.ReceiveShutdown`
  ;[1 0.09375 0.09375 0.26] Handle game shutdown
  (`self.OnShutdown`))

(event `OnShutdown`
  (bind _rememberuser (`self.RememberUser`))
  (`|ExecutionSequence`
    (:`then_0`
      (bind _returnvalue (`BCWrapperProxy.GetStoredAnonymousId` null))
      (`KismetSystemLibrary.PrintString` (`KismetStringLibrary.Concat_StrStr` "Stored Anonymous ID: " _returnvalue)))
    (:`then_1`
      (bind _returnvalue_2 (`BCWrapperProxy.GetStoredProfileId` null))
      (`KismetSystemLibrary.PrintString` (`KismetStringLibrary.Concat_StrStr` "Stored Profile ID: " _returnvalue_2)))
    (:`then_2`
      ;[1 0.09375 0.09375 0.26] Handle game shutdown
      (`KismetSystemLibrary.PrintString` (`KismetStringLibrary.Concat_StrStr` "[OnShutdown] RememberUser? " (`KismetStringLibrary.Conv_BoolToString` _rememberuser)))
      (`|ExecutionSequence`
        (:`then_0`
          (bind _returnvalue_3 (`BCRelayProxy.IsConnected` null))
          (if _returnvalue_3
            (`BCRelayProxy.Disconnect` null)))
        (:`then_1`
          (`|BrainCloudCall` null (not _rememberuser)))))))

(event `OnBCInitialized`
  ;[0.3698 0.3794 0.6771 0.688] Initialize and Run brainCloud
  (if (`self.brainCloudInitialized`)
    (`BCClientProxy.RunCallbacks` (`self.brainCloudWrapper`))))

(event `SetupRTT`
  ;[0.8542 0.539 0.3515 0.214] Setup RTT
  (`self.EnableRTT`
    (:`OnSuccess`
      (bind _jsondata (`|BrainCloudCall` null)
        (:`then`
          (`|BrainCloudCall` null "all" true
            (:`OnSuccess`
              (`|BrainCloudCall` null true))))
        (:`OnRTTCallback`
          (`self.OnRTTPresence` _jsondata))))))

(event `LogoutUser`
  ;[1 0.09375 0.09375 0.26] Logout
  (`BCRTTProxy.DeregisterAllRTTCallbacks` null)
  (`BCRTTProxy.DisableRTT` (`self.brainCloudWrapper`))
  (`|BrainCloudCall` null true
    (:`OnSuccess`
      (`self.SwitchUIScreen` "NewEnumerator0")
      (`self.ChangeUIState` "NewEnumerator0"))))

(event `LeaveLobby`
  ;[1 0.09375 0.09375 0.26] Leave Lobby
  (bind _jsondata (`|BrainCloudCall` null (`.LobbyId_3_42B89D4145E9656634409B9C455E773B` (break `/Game/Blueprints/Core/Data/LobbyData` (`self.LobbyData`))))
    (:`OnSuccess`
      (`self.SwitchUIScreen` "NewEnumerator1")
      (`self.ChangeUIState` "NewEnumerator0"))
    (:`OnFailure`
      (`self.OnFailureCallback` _jsondata))))

(event `CancelFindRequest`
  ;[1 0.2552 0.2552 0.219] Cancel Find Request
  (`|BrainCloudCall` null (`self.CurrentLobbySearch`)
    (:`OnSuccess`
      (set `self.CurrentLobbySearch` "")
      (`self.ChangeUIState` "NewEnumerator0"))))

(event `CreateLobby`
  (bind _lobbytype (`self.LobbyType`))
  ;[0.3873 0.4415 1 0.255] Create Lobby
  (`self.ChangeUIState` "NewEnumerator2")
  (bind _jsondata (`|BrainCloudCall` null)
    (:`then`
      (`|BrainCloudCall` null _lobbytype 0 2 false "{}" "all" "{}" (`|MakeArray`)
        (:`then`
          (set `self.CurrentLobbySearch` _lobbytype))))
    (:`OnRTTCallback`
      (bind _room_ready (`self.HandleLobbyCallbacks` _jsondata))
      (if _room_ready
        (`self.Connect to Server`)))))

(event `JoinLobby`
  (params (LobbyID :type String))
  ;[0.5313 0.2825 1 0.645] Join Lobby
  (`self.ChangeUIState` "NewEnumerator1")
  (bind _jsondata (`|BrainCloudCall` null)
    (:`then`
      (`|BrainCloudCall` null LobbyID false "{}" "all" (`|MakeArray`)))
    (:`OnRTTCallback`
      (bind _room_ready (`self.HandleLobbyCallbacks` _jsondata))
      (if _room_ready
        (`self.Connect to Server`)))))

(event `FindLobby`
  (bind _lobbytype (`self.LobbyType`))
  ;[0.3873 0.4415 1 0.255] Find Lobby
  (`self.ChangeUIState` "NewEnumerator1")
  (bind _jsondata (`|BrainCloudCall` null)
    (:`then`
      (`|BrainCloudCall` null _lobbytype 0 1 "{ \n    \"strategy\": \"ranged-absolute\", \n    \"alignment\": \"center\", \n    \"ranges\": [ \n        5, \n        7.5, \n        10 \n    ] \n}" "{}" 0 false "{}" "all" "{}" (`|MakeArray`)
        (:`then`
          (set `self.CurrentLobbySearch` _lobbytype))))
    (:`OnRTTCallback`
      (bind _room_ready (`self.HandleLobbyCallbacks` _jsondata))
      (if _room_ready
        (`self.Connect to Server`)))))

(event `UpdateLobbyReady`
  (params (ready :type Boolean))
  (`|BrainCloudCall` null (`.LobbyId_3_42B89D4145E9656634409B9C455E773B` (break `/Game/Blueprints/Core/Data/LobbyData` (`self.LobbyData`))) ready "{}"))

(event `UpdateLobbyType`
  (params (newLobbyType :type String))
  (set `self.LobbyType` newLobbyType))

(fn `ChangeUIState`
  (params (newState :type "/Game/Blueprints/Core/Data/UIState Enum" :default "NewEnumerator0"))
  (`/Game/Blueprints/UI/WBP_GameMenu.ChangeState` (`self.MainUIWidget`) newState))

(fn `Connect to Server`
  (bind (_roomdata_lobbyid _roomdata_address _roomdata_portudp) (break `/Game/Blueprints/Core/Data/RoomData` (`self.RoomData`)))
  (`self.ChangeUIState` "NewEnumerator8")
  (`KismetSystemLibrary.ExecuteConsoleCommand` (`KismetStringLibrary.Concat_StrStr` "open " _roomdata_address ":" (`KismetStringLibrary.Conv_IntToString` _roomdata_portudp)) null))

(fn `GetLobbyMember`
  (params (cxId :type String))
  (returns (LobbyMemberData :type "/Game/Blueprints/Core/Data/LobbyMemberData Structure") (Found :type Boolean))
  (for _array_element (`.Members_23_F310257D4A29316BF1E3278B40E1ECB0` (break `/Game/Blueprints/Core/Data/LobbyData` (`self.LobbyData`)))
    (if (`KismetStringLibrary.EqualEqual_StrStr` (`.CxId_17_921E40064DDD89563539C68EFFCA3E6F` (break `/Game/Blueprints/Core/Data/LobbyMemberData` _array_element)) cxId)
      (return _array_element true)))
  (return (struct) false))

(fn `GetUIState`)

(fn `HandleLobbyCallbacks`
  (params (jsonDataString :type String))
  (returns (`Room Ready` :type Boolean))
  (locals (LobbyJsonData :type "JsonObjectWrapper Structure"))
  (bind _lobbyjsondata (`local.LobbyJsonData`))
  (bind _outjsonobject (`JsonBlueprintFunctionLibrary.FromString` jsonDataString))
  (bind _output_get (set `local.LobbyJsonData` _outjsonobject))
  (`self.ProcessRTTLobbyOp` _output_get
    (:`MEMBER JOIN`
      (`self.SetLobbyData` _lobbyjsondata)
      (bind _outvalue (`|GetJsonField` _lobbyjsondata "data"))
      (bind _outvalue_2 (`|GetJsonField` _outvalue "member"))
      (bind _outvalue_3 (`|GetJsonField` _outvalue_2 "profileId"))
      (`self.OnLobbyMemberJoined` _outvalue_2)
      (`self.IsLocalPlayer` _outvalue_3
        (:`Is Local Player`
          (`self.OnJoinedLobby`)
          (`self.SwitchUIScreen` "NewEnumerator2")
          (`self.ChangeUIState` "NewEnumerator3"))
        (:`Is Remote Player`
          (`self.OnLobbyUpdate`)))
      (return false))
    (:`MEMBER UPDATE`
      (`self.SetLobbyData` _lobbyjsondata :!label _label)
      (`self.OnLobbyUpdate`)
      (return false))
    (:`MEMBER LEFT`
      (goto _label))
    (:`STARTING`
      (`self.ChangeUIState` "NewEnumerator6"))
    (:`ROOM ASSIGNED`
      (`self.SetRoomData` (`local.LobbyJsonData`))
      (`self.ChangeUIState` "NewEnumerator7")
      (return false))
    (:`ROOM READY`
      (`self.SetRoomData` (`local.LobbyJsonData`))
      (`WidgetBlueprintLibrary.SetInputMode_GameOnly` (`GameplayStatics.GetPlayerController` 0))
      (return true))
    (:`DISBANDED`
      (bind _errormessage (`self.ProcessLobbyErrorMessage` (`local.LobbyJsonData`)))
      (`self.ChangeUIState` "NewEnumerator0")
      (`self.OnFailureCallback` _errormessage)
      (`self.SwitchUIScreen` "NewEnumerator1")
      (return false))
    (:`DEFAULT`
      (return false))))

(fn `InitializeBrainCloud`
  (`/Engine/EditorBlueprintResources/StandardMacros.IsValid` (`self.brainCloudWrapper`)
    (:`Is Not Valid`
      (bind _returnvalue (`BCWrapperProxy.CreateBrainCloudWrapper` ""))
      (bind _output_get (set `self.brainCloudWrapper` _returnvalue))
      (`BCWrapperProxy.SetDefaultBrainCloudInstance` _output_get)
      (bind _returnvalue_2 (`BrainCloudFunctionLibrary.GetBCAppData`))
      (bind (_serverurl _appid _appsecret _version) (break `BrainCloudAppDataStruct` _returnvalue_2))
      (`BCClientProxy.Initialize` _output_get _serverurl _appsecret _appid _version)
      (bind _returnvalue_3 (`BCClientProxy.IsInitialized` (`self.brainCloudWrapper`)))
      (if _returnvalue_3
        (`BCClientProxy.EnableLogging` null true)
        (set `self.brainCloudInitialized` true)
        (else
          (`KismetSystemLibrary.PrintString` "ERROR: Cannot initialize BrainCloud." true true (struct :`R` 1.0 :`B` 0.044729 :`A` 1.0)))))))

(fn `OnFailureCallback`
  (params (errorMessage :type String))
  (bind _outjsonobject (`JsonBlueprintFunctionLibrary.FromString` errorMessage))
  (bind _outvalue (`|GetJsonField` _outjsonobject "reason_code"))
  (if (not (`KismetStringLibrary.EqualEqual_StrStr` "80300" _outvalue))
    (`/Game/Blueprints/UI/WBP_GameMenu.ShowError` (`self.MainUIWidget`) errorMessage))
  (return))

(fn `ProcessLobbyData`
  (params (data :type "JsonObjectWrapper Structure"))
  (returns (`lobby data` :type "/Game/Blueprints/Core/Data/LobbyData Structure"))
  (locals (m_lobbyMembers :type "Array of /Game/Blueprints/Core/Data/LobbyMemberData Structure"))
  (bind _m_lobbymembers (`local.m_lobbyMembers`))
  (`KismetArrayLibrary.Array_Clear` (`local.m_lobbyMembers`))
  (bind _outvalue (`|GetJsonField` data "data"))
  (bind _outvalue_2 (`|GetJsonField` _outvalue "lobbyId"))
  (bind _outvalue_3 (`|GetJsonField` _outvalue "lobby"))
  (bind _outvalue_4 (`|GetJsonField` _outvalue_3 "state"))
  (bind _outvalue_5 (`|GetJsonField` _outvalue_3 "rating"))
  (bind _outvalue_6 (`|GetJsonField` _outvalue_3 "lobbyTypeDef"))
  (bind _outvalue_7 (`|GetJsonField` _outvalue_6 "lobbyTypeId"))
  (bind _outvalue_8 (`|GetJsonField` _outvalue_6 "teams"))
  (bind _outvalue_9 (`|GetJsonField` _outvalue_8 "all"))
  (bind _outvalue_10 (`|GetJsonField` _outvalue_9 "minUsers"))
  (bind _outvalue_11 (`|GetJsonField` _outvalue_9 "maxUsers"))
  (bind _outvalue_12 (`|GetJsonField` _outvalue_3 "members"))
  (for _array_element _outvalue_12
    (bind _member_data (`self.ProcessLobbyMemberData` _array_element))
    (`KismetArrayLibrary.Array_Add` _m_lobbymembers _member_data))
  (bind _outvalue_13 (`|GetJsonField` _outvalue_3 "ownerCxId"))
  (return (make `/Game/Blueprints/Core/Data/LobbyData` _outvalue_2 _outvalue_4 _outvalue_5 _outvalue_7 _outvalue_10 _outvalue_11 _outvalue_13 _m_lobbymembers)))

(fn `ProcessLobbyErrorMessage`
  (params (data :type "JsonObjectWrapper Structure"))
  (returns (ErrorMessage :type String))
  (bind _outvalue (`|GetJsonField` data "data"))
  (bind _outvalue_2 (`|GetJsonField` _outvalue "reason"))
  (bind _outvalue_3 (`|GetJsonField` _outvalue_2 "desc"))
  (return _outvalue_3))

(fn `ProcessLobbyMemberData`
  (params (data :type "JsonObjectWrapper Structure"))
  (returns (`member data` :type "/Game/Blueprints/Core/Data/LobbyMemberData Structure"))
  (bind _outjsonstring (`JsonBlueprintFunctionLibrary.ToString` data))
  (`KismetSystemLibrary.LogString` (`KismetStringLibrary.Concat_StrStr` "Processing lobby member data:  \n" _outjsonstring))
  (bind _outvalue (`|GetJsonField` data "profileId"))
  (bind _outvalue_2 (`|GetJsonField` data "name"))
  (bind _outvalue_3 (`|GetJsonField` data "pic"))
  (bind _outvalue_4 (`|GetJsonField` data "rating"))
  (bind _outvalue_5 (`|GetJsonField` data "isReady"))
  (bind _outvalue_6 (`|GetJsonField` data "extra"))
  (bind _outvalue_7 (`|GetJsonField` data "cxId"))
  (bind _outvalue_8 (`|GetJsonField` data "passcode"))
  (bind _returnvalue (`BCClientProxy.GetProfileId` null))
  (if (`KismetStringLibrary.EqualEqual_StrStr` _returnvalue _outvalue)
    (bind _lobbymemberdata (make `/Game/Blueprints/Core/Data/LobbyMemberData` _outvalue _outvalue_2 _outvalue_3 _outvalue_4 _outvalue_5 _outvalue_6 _outvalue_7 _outvalue_8))
    (setmembers `/Game/Blueprints/Core/Data/PlayerData` :`StructRef` (`self.PlayerData`) :`LobbyMemberData` _lobbymemberdata))
  (return _lobbymemberdata))

(fn `ProcessPlayerData`
  (params (data :type "JsonObjectWrapper Structure"))
  (returns (`player data` :type "/Game/Blueprints/Core/Data/PlayerData Structure"))
  (bind _outvalue (`|GetJsonField` data "data"))
  (bind _outvalue_2 (`|GetJsonField` _outvalue "playerName"))
  (bind _outvalue_3 (`|GetJsonField` _outvalue "emailAddress"))
  (bind _outvalue_4 (`|GetJsonField` _outvalue "id"))
  (bind _outvalue_5 (`|GetJsonField` _outvalue "experiencePoints"))
  (bind _outvalue_6 (`|GetJsonField` _outvalue "experienceLevel"))
  (bind _outvalue_7 (`|GetJsonField` _outvalue "pictureUrl"))
  (bind _outvalue_8 (`|GetJsonField` _outvalue "statistics"))
  (return (make `/Game/Blueprints/Core/Data/PlayerData` _outvalue_4 _outvalue_2 _outvalue_3 _outvalue_7 _outvalue_5 _outvalue_6 _outvalue_8)))

(fn `ProcessRoomData`
  (params (data :type "JsonObjectWrapper Structure"))
  (returns (`room data` :type "/Game/Blueprints/Core/Data/RoomData Structure"))
  (bind _lobbydata (`self.LobbyData`))
  (bind _outvalue (`|GetJsonField` data "data"))
  (bind _outvalue_2 (`|GetJsonField` _outvalue "lobbyId"))
  (bind _outvalue_3 (`|GetJsonField` _outvalue "connectData"))
  (bind _outvalue_4 (`|GetJsonField` _outvalue "passcode"))
  (bind _outvalue_5 (`|GetJsonField` _outvalue_3 "address"))
  (bind _outvalue_6 (`|GetJsonField` _outvalue_3 "ports"))
  (bind _outvalue_7 (`|GetJsonField` _outvalue_6 "7777/udp"))
  (if (`KismetStringLibrary.EqualEqual_StrStr` _outvalue_2 (`.LobbyId_3_42B89D4145E9656634409B9C455E773B` (break `/Game/Blueprints/Core/Data/LobbyData` _lobbydata)))
    (bind _roomdata (make `/Game/Blueprints/Core/Data/RoomData` _outvalue_2 _outvalue_5 _outvalue_7 0 _outvalue_4))
    (setmembers `/Game/Blueprints/Core/Data/LobbyData` :`StructRef` _lobbydata :`roomData` _roomdata))
  (return _roomdata))

(fn `ResetData`
  (`BCWrapperProxy.ResetStoredAnonymousId` null)
  (`BCWrapperProxy.ResetStoredProfileId` null)
  (set `self.PlayerData` (struct))
  (set `self.LobbyData` (struct))
  (set `self.RoomData` (struct)))

(fn `SetLobbyData`
  (params (jsonData :type "JsonObjectWrapper Structure"))
  (bind _lobby_data (`self.ProcessLobbyData` jsonData))
  (set `self.LobbyData` _lobby_data))

(fn `SetPlayerData`
  (params (JsonDataString :type String))
  (bind _outjsonobject (`JsonBlueprintFunctionLibrary.FromString` JsonDataString))
  (bind _player_data (`self.ProcessPlayerData` _outjsonobject))
  (set `self.PlayerData` _player_data))

(fn `SetRoomData`
  (params (JsonData :type "JsonObjectWrapper Structure"))
  (bind _room_data (`self.ProcessRoomData` JsonData))
  (set `self.RoomData` _room_data))

(fn `SwitchUIScreen`
  (params (UIScreen :type "/Game/Blueprints/Core/Data/UIScreens Enum" :default "NewEnumerator0"))
  (`/Game/Blueprints/UI/WBP_GameMenu.SwitchScreen` (`self.MainUIWidget`) UIScreen))

(fn `ToggleLoadingScreen`
  (params (enabled :type Boolean) (LoadingMessage :type String))
  (bind _mainuiwidget (`self.MainUIWidget`))
  (`/Engine/EditorBlueprintResources/StandardMacros.IsValid` _mainuiwidget
    (:`Is Valid`
      (`/Game/Blueprints/UI/WBP_GameMenu.ToggleLoadingScreen` _mainuiwidget enabled LoadingMessage))))

(fn `UpdatePlayerName`
  (params (NewName :type String))
  (setmembers `/Game/Blueprints/Core/Data/PlayerData` :`StructRef` (`self.PlayerData`) :`Name` NewName))